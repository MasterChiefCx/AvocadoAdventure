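; Test combatant Blueprint for a timed turn-based combat system, with health, mana and damage.
; On BeginPlay it fills health and mana from their maximums and caches the level's BP_CombatSystem.
; Tick fills a time gauge; once past its maximum, the character passes itself to the combat system as turn or next character, depending on that system's flags.
; Damage functions expose its attack value and subtract health, printing "dead" below one.
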(event `self.ReceiveBeginPlay`
  (`self.SetStats`)
  (bind _returnvalue (`GameplayStatics.GetActorOfClass` "/Game/AvocadoAdventure/CombatSystem/BP_CombatSystem.BP_CombatSystem_C"))
  (set `self.CombatSystem` _returnvalue))

(event `self.ReceiveTick`
  (params (DeltaSeconds :type "Float (single-precision)"))
  (`self.Time` DeltaSeconds))

(fn `GetDamage`
  (returns (_damage :type Integer))
  ;[1 1 1] Hacer Daño
  (return (`self.Damage`)))

(fn `ReciveDamage`
  (params (Damage :type Integer))
  ;[1 1 1] Recibir Daño
  (bind _output_get (set `self.Health` (- (`self.Health`) Damage)))
  (if (< _output_get 1)
    (`KismetSystemLibrary.PrintString` "dead")))

(fn `SetStats`
  ;[1 1 1] Funcion para setear la vida y mana
  (set `self.Health` (`self.MaxHealth`))
  (set `self.Mana` (`self.MasxMana`)))

(fn `Time`
  (params (_time :type "Float (double-precision)"))
  (bind _combatsystem (`self.CombatSystem`))
  (bind _currenttime (`self.CurrentTime`))
  ;[1 1 1] Funcion de Tiempo
  (if (<= _currenttime (`self.MaxTime`))
    (set `self.CurrentTime` (+ _time _currenttime))
    (elif (`/Game/AvocadoAdventure/CombatSystem/BP_CombatSystem.NexChar` _combatsystem)
      (set `self.CurrentChar` false)
      (`/Game/AvocadoAdventure/CombatSystem/BP_CombatSystem.PlayerTurn` _combatsystem self)
      (elif (`/Game/AvocadoAdventure/CombatSystem/BP_CombatSystem.NexChar2` _combatsystem)
        (if (not (== self (`/Game/AvocadoAdventure/CombatSystem/BP_CombatSystem.CurrentCharacter` _combatsystem)))
          (`/Game/AvocadoAdventure/CombatSystem/BP_CombatSystem.NextCharFunc` _combatsystem self))))))

(fn `UserConstructionScript`)