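; BP_Enemy is an enemy in the combat system that tracks health, an animation state and an attack timer.
; On begin play it fills its health and caches BP_CombatSystem.
; While the game instance's OnFight flag is set, Tick advances the timer and calls EnemyAttack on the combat system once it is full, without resetting it here.
; DealDamage subtracts health, switches animation state and reports death below zero, while Die is an empty stub.
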(event `self.ReceiveBeginPlay`
  (`self.SetStats`)
  (bind _returnvalue (`GameplayStatics.GetActorOfClass` "/Game/AvocadoAdventure/CombatSystem/BP_CombatSystem.BP_CombatSystem_C"))
  (set `self.BP_CombatSystem` _returnvalue)
  (set `self.AnimState` 0))

(event `self.ReceiveTick`
  (params (DeltaSeconds :type "Float (single-precision)"))
  (bind _asmy_game_instance (cast `/Game/AvocadoAdventure/CombatSystem/MyGameInstance` (`GameplayStatics.GetGameInstance`)))
  (if (`/Game/AvocadoAdventure/CombatSystem/MyGameInstance.OnFight` _asmy_game_instance)
    (`self.TimeFunc` DeltaSeconds)))

(fn `DealDamage`
  (params (_damage :type Integer))
  (returns (_isdead :type Boolean))
  (bind _currenthealth (`self.CurrentHealth`))
  (bind _returnvalue (< _currenthealth 0))
  (set `self.AnimState` 2)
  (set `self.CurrentHealth` (- _currenthealth _damage))
  (if _returnvalue
    (set `self.AnimState` 3))
  (return _returnvalue))

(fn `Die`)

(fn `SetStats`
  (set `self.CurrentHealth` (`self.MaxHealth`)))

(fn `TimeFunc`
  (params (_time :type "Float (double-precision)"))
  (bind _currenttime (`self.CurrentTime`))
  (if (< _currenttime (`self.MaxTime`))
    (set `self.CurrentTime` (+ _currenttime _time))
    (else
      (set `self.AnimState` 1)
      (set `self.AnimState` 0)
      (`/Game/AvocadoAdventure/CombatSystem/BP_CombatSystem.EnemyAttack` (`self.BP_CombatSystem`) self))))

(fn `UserConstructionScript`)