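; BP_InputManager is an actor that maps keyboard input to attacks in the combat system.
; On BeginPlay it finds the BP_CombatSystem actor in the level and caches a reference to it.
; Pressing number keys 1, 2 or 3 calls MakeDamageToEnemy on that reference with a matching zero-based index.
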(event `self.ReceiveBeginPlay`
  (bind _returnvalue (`GameplayStatics.GetActorOfClass` "/Game/AvocadoAdventure/CombatSystem/BP_CombatSystem.BP_CombatSystem_C"))
  (set `self.BP_CombatSystem` _returnvalue))

(event `Key|One`
  (params (Key :type "Key Structure"))
  (:`Pressed`
    (bind _output_get (set `self.index` 0))
    (`/Game/AvocadoAdventure/CombatSystem/BP_CombatSystem.MakeDamageToEnemy` (`self.BP_CombatSystem`) _output_get)))

(event `Key|Two`
  (params (Key :type "Key Structure"))
  (:`Pressed`
    (bind _output_get (set `self.index` 1))
    (`/Game/AvocadoAdventure/CombatSystem/BP_CombatSystem.MakeDamageToEnemy` (`self.BP_CombatSystem`) _output_get)))

(event `Key|Three`
  (params (Key :type "Key Structure"))
  (:`Pressed`
    (bind _output_get (set `self.index` 2))
    (`/Game/AvocadoAdventure/CombatSystem/BP_CombatSystem.MakeDamageToEnemy` (`self.BP_CombatSystem`) _output_get)))

(fn `UserConstructionScript`)