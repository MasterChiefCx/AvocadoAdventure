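; BP_CombatSystem sets up the combat UI and exposes turn hooks for a player-versus-enemy battle.
; On BeginPlay it creates the WB_Characters widget, gathers every BP_TestCharacter in the level and takes the stat widgets and panel buttons from that widget.
; Each stat widget is bound to a character by matching array index.
; PlayerTurn and EnemyTurn simply forward to the widget, with no turn logic here.
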(event `self.ReceiveBeginPlay`
  (`self.GetReferences`)
  (`self.SetStatsUI`))

(fn `EnemyTurn`
  (`/Game/AvocadoAdventure/CombatSystem/UI_CombatSystem/WB_Characters.EnemyTurn` (`self.WB_Chars`)))

(fn `GetReferences`
  (bind _returnvalue (`|CreateWidget` "/Game/AvocadoAdventure/CombatSystem/UI_CombatSystem/WB_Characters.WB_Characters_C"))
  (bind _output_get (set `self.WB_Chars` _returnvalue))
  (`UserWidget.AddToViewport` _output_get 0)
  (bind _outactors (`GameplayStatics.GetAllActorsOfClass` "/Game/AvocadoAdventure/CombatSystem/BP_TestCharacter.BP_TestCharacter_C"))
  (set `self.Characters` _outactors)
  (bind (_arrychars __panelbuttons) (`/Game/AvocadoAdventure/CombatSystem/UI_CombatSystem/WB_Characters.SetArryCharStats` (`self.WB_Chars`)))
  (set `self.CharStats` _arrychars)
  (set `self.PanelButtons` __panelbuttons))

(fn `PlayerTurn`
  (`/Game/AvocadoAdventure/CombatSystem/UI_CombatSystem/WB_Characters.PlayerTurn` (`self.WB_Chars`)))

(fn `SetStatsUI`
  (for (_array_element _array_index) (`self.CharStats`)
    (`/Game/AvocadoAdventure/CombatSystem/UI_CombatSystem/WB_CharacterStats.SetStats` _array_element (`|GetArrayItem` (`self.Characters`) _array_index))))

(fn `UserConstructionScript`)