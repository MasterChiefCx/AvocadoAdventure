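; Collectible flyer (Folleto) pickup that stays collected across sessions through a SaveStats save in slot "1".
; On BeginPlay it loads or creates the save and destroys itself if its CollIndex entry in the Collectors array is true.
; When the player overlaps its box, it increments the Folletos count, saves that entry as true, plays a sound, briefly pulses the player's TakeFolleto flag and destroys itself.
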(event `self.ReceiveBeginPlay`
  (bind _asbp_player (cast `/Game/AvocadoAdventure/Character/BP_Player` (`GameplayStatics.GetPlayerCharacter` 0)))
  (set `self.Player` _asbp_player)
  (bind _savestats (`self.SaveGaameInit`))
  (`self.DesactivarActor` _savestats))

(event `self.BoxColision.OnComponentBeginOverlap`
  (params (OverlappedComponent :type "PrimitiveComponent Object Reference") (OtherActor :type "Actor Object Reference") (OtherComp :type "PrimitiveComponent Object Reference") (OtherBodyIndex :type Integer) (bFromSweep :type Boolean) (SweepResult :type "HitResult Structure (by ref)"))
  (bind _player (`self.Player`))
  (bind _asbp_player (cast `/Game/AvocadoAdventure/Character/BP_Player` OtherActor))
  (set `/Game/AvocadoAdventure/Character/BP_Player.Folletos` (+ (`/Game/AvocadoAdventure/Character/BP_Player.Folletos` _asbp_player) 1) _asbp_player)
  (bind _savestats (`self.SaveGaameInit`))
  (`self.SetearFolleto` _savestats)
  (`GameplayStatics.PlaySound2D` "/Game/AvocadoAdventure/StagesAssets/Collectionables/pickupCoin.pickupCoin" 1.0 1.0 0.0 null null)
  (set `/Game/AvocadoAdventure/Character/BP_Player.TakeFolleto` true _player)
  (`KismetSystemLibrary.Delay` 0.2)
  (set `/Game/AvocadoAdventure/Character/BP_Player.TakeFolleto` false _player)
  (`self.K2_DestroyActor`))

(fn `DesactivarActor`
  (params (_SaveStats :type "/Game/AvocadoAdventure/CombatSystem/SaveStats Object Reference"))
  (for (_array_element _array_index) (`/Game/AvocadoAdventure/CombatSystem/SaveStats.Collectors` _SaveStats)
    (if (== _array_index (`self.CollIndex`))
      (`KismetSystemLibrary.PrintString` "Index")
      (if _array_element
        (`KismetSystemLibrary.PrintString` "Folleto")
        (`self.K2_DestroyActor`)))))

(fn `SaveGaameInit`
  (returns (SaveStats :type "/Game/AvocadoAdventure/CombatSystem/SaveStats Object Reference"))
  (bind _returnvalue (`GameplayStatics.DoesSaveGameExist` "1"))
  (if _returnvalue
    (bind _returnvalue_2 (`GameplayStatics.LoadGameFromSlot` "1"))
    (bind _assave_stats (cast `/Game/AvocadoAdventure/CombatSystem/SaveStats` _returnvalue_2))
    (return _assave_stats)
    (else
      (bind _returnvalue_3 (`GameplayStatics.CreateSaveGameObject` "/Game/AvocadoAdventure/CombatSystem/SaveStats.SaveStats_C"))
      (return _returnvalue_3))))

(fn `SetearFolleto`
  (params (_Savestats :type "/Game/AvocadoAdventure/CombatSystem/SaveStats Object Reference"))
  (`KismetArrayLibrary.Array_Set` (`/Game/AvocadoAdventure/CombatSystem/SaveStats.Collectors` _Savestats) (`self.CollIndex`) true)
  (`GameplayStatics.SaveGameToSlot` _Savestats "1"))

(fn `UserConstructionScript`)